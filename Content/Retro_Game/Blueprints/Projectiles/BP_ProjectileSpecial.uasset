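; BP_ProjectileSpecial is a special projectile that deals a small amount of damage to actors it overlaps, ignoring BP_CharacterBase.
; On a valid overlap it switches its flipbook to the impact animation, applies damage, disables sphere collision and stops projectile movement.
; It then waits for the length of the impact flipbook before destroying itself, so the animation plays out in full.
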(event `self.ReceiveActorBeginOverlap`
  (params (OtherActor :type "Actor Object Reference"))
  (bind _f_projectile (`self.F_Projectile`))
  (if (!= OtherActor "/Game/Retro_Game/Blueprints/BP_CharacterBase.BP_CharacterBase")
    (`PaperFlipbookComponent.SetFlipbook` _f_projectile "/Game/Retro_Game/Sprites/FlipBooks/Projectile/F_ProjectileImpact.F_ProjectileImpact")
    (`GameplayStatics.ApplyDamage` OtherActor 0.2)
    (`PrimitiveComponent.SetCollisionEnabled` (`self.Sphere`) "NoCollision")
    (`MovementComponent.StopMovementImmediately` (`self.ProjectileMovement`))
    (`KismetSystemLibrary.Delay` (`PaperFlipbookComponent.GetFlipbookLength` _f_projectile))
    (`self.K2_DestroyActor`)))

(fn `UserConstructionScript`)