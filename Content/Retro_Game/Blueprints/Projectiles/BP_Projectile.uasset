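; Projectile actor for a retro game that deals a small fixed amount of damage to what it hits.
; A sphere overlap with anything other than BP_CharacterBase swaps the Paper2D flipbook to an impact animation and applies damage.
; It then disables sphere collision, halts the projectile movement component, and destroys itself after a delay matching the flipbook's length.
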(event `self.Sphere.OnComponentBeginOverlap`
  (params (OverlappedComponent :type "PrimitiveComponent Object Reference") (OtherActor :type "Actor Object Reference") (OtherComp :type "PrimitiveComponent Object Reference") (OtherBodyIndex :type Integer) (bFromSweep :type Boolean) (SweepResult :type "HitResult Structure (by ref)"))
  (bind _f_projectile (`self.F_Projectile`))
  (if (!= OtherActor "/Game/Retro_Game/Blueprints/BP_CharacterBase.BP_CharacterBase")
    (`PaperFlipbookComponent.SetFlipbook` _f_projectile "/Game/Retro_Game/Sprites/FlipBooks/Projectile/F_ProjectileImpact.F_ProjectileImpact")
    (`GameplayStatics.ApplyDamage` OtherActor 0.2)
    (`PrimitiveComponent.SetCollisionEnabled` (`self.Sphere`) "NoCollision")
    (`MovementComponent.StopMovementImmediately` (`self.ProjectileMovement`))
    (`KismetSystemLibrary.Delay` (`PaperFlipbookComponent.GetFlipbookLength` _f_projectile))
    (`self.K2_DestroyActor`)))

(fn `UserConstructionScript`)