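; BP_Barrel is a barrel cannon for a Paper2D level that captures the player character and fires it out along an arrow.
; On overlap it hides and freezes the character at the arrow, disabling damage, firing and double jump.
; Tick polls for jump input, then launches the character, plays sound and explosion flipbook, and restores abilities, some after the animation.
; A DoOnce, reset on each overlap, limits it to one shot per entry.
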(event `self.ReceiveTick`
  (params (DeltaSeconds :type "Float (single-precision)"))
  (bind _returnvalue (`GameplayStatics.GetPlayerController` 0))
  (bind _paperflipbook (`self.PaperFlipbook`))
  ;[1 1 1] Watch for jump button pressed
  (if (or (`PlayerController.WasInputKeyJustPressed` _returnvalue "SpaceBar") (`PlayerController.WasInputKeyJustPressed` _returnvalue "Gamepad_FaceButton_Bottom"))
    (`/Engine/EditorBlueprintResources/StandardMacros.DoOnce` false :!label _label
      (:`Completed`
        ;[1 1 1] Shoot out
        (`/Engine/EditorBlueprintResources/StandardMacros.IsValid` (stale `self.ReceiveActorBeginOverlap` _asbp_character_base)
          (:`Is Valid`
            (`Character.LaunchCharacter` (stale `self.ReceiveActorBeginOverlap` _asbp_character_base) (* (`KismetMathLibrary.Conv_RotatorToVector` (`SceneComponent.K2_GetComponentRotation` (`self.Arrow`))) (`self.Force`)) false true)
            (`GameplayStatics.PlaySoundAtLocation` "/Game/Retro_Game/Sounds/SFX_GotHit_v2_Cue.SFX_GotHit_v2_Cue" (`self.K2_GetActorLocation`) (struct) 1.0 1.0 0.0 null null null null)
            (`self.SetActorHiddenInGame` (stale `self.ReceiveActorBeginOverlap` _asbp_character_base) false)
            (set `CharacterMovementComponent.MaxFlySpeed` 600.0 (`Character.CharacterMovement` (stale `self.ReceiveActorBeginOverlap` _asbp_character_base)))
            (`PaperFlipbookComponent.SetFlipbook` _paperflipbook "/Game/Retro_Game/Sprites/FlipBooks/Explosion/F_Explosion.F_Explosion")
            (set `Actor.bCanBeDamaged` true (stale `self.ReceiveActorBeginOverlap` _asbp_character_base))
            (`KismetSystemLibrary.Delay` (`PaperFlipbookComponent.GetFlipbookLength` _paperflipbook))
            (`PaperFlipbookComponent.SetFlipbook` _paperflipbook null)
            (set `/Game/Retro_Game/Blueprints/BP_CharacterBase.bCanFire` true (stale `self.ReceiveActorBeginOverlap` _asbp_character_base))
            (set `/Game/Retro_Game/Blueprints/BP_CharacterBase.bCanDoubleJumpTempOverride` true (stale `self.ReceiveActorBeginOverlap` _asbp_character_base))))))))

(event `self.ReceiveActorBeginOverlap`
  (params (OtherActor :type "Actor Object Reference"))
  (`|ExecutionSequence`
    (:`then_0`
      (goto _label :!via `Reset`))
    (:`then_1`
      (bind _asbp_character_base (cast `/Game/Retro_Game/Blueprints/BP_CharacterBase` OtherActor))
      ;[1 1 1] Inside barrel
      (set `/Game/Retro_Game/Blueprints/BP_CharacterBase.bCanDoubleJumpTempOverride` false _asbp_character_base)
      (set `/Game/Retro_Game/Blueprints/BP_CharacterBase.bCanFire` false _asbp_character_base)
      (set `Actor.bCanBeDamaged` false _asbp_character_base)
      (bind _charactermovement (`Character.CharacterMovement` _asbp_character_base))
      (`CharacterMovementComponent.SetMovementMode` _charactermovement "MOVE_Flying" 0)
      (`self.SetActorHiddenInGame` _asbp_character_base true)
      (`MovementComponent.StopMovementImmediately` _charactermovement)
      (set `CharacterMovementComponent.MaxFlySpeed` 0.0 _charactermovement)
      (`self.K2_TeleportTo` :`self` _asbp_character_base :`DestLocation` (`SceneComponent.K2_GetComponentLocation` (`self.Arrow`))))))

(fn `UserConstructionScript`)