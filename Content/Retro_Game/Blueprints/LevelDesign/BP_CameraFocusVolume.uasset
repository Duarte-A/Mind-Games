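; BP_CameraFocusVolume is a level-design trigger volume that switches the view to its own camera while the player character is inside.
; Overlap events blend the view target to the volume on entry and back to the character on exit.
; An optional spawn flag makes Tick check the overlap and snap the view once when the player starts inside.
; The construction script applies exposed box scale, camera position and orthographic width.
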(event `self.ReceiveBeginPlay`
  (bind _asbp_character_base (cast `/Game/Retro_Game/Blueprints/BP_CharacterBase` (`GameplayStatics.GetPlayerCharacter` 0)))
  (set `self.PlayerCast` _asbp_character_base))

(event `self.ReceiveTick`
  (params (DeltaSeconds :type "Float (single-precision)"))
  (if (`self.PlayerSpawnsInThisVolume`)
    (`self.ForceFocusOnFirstSpawn`)))

(event `self.ReceiveActorBeginOverlap`
  (params (OtherActor :type "Actor Object Reference"))
  (bind _returnvalue (`GameplayStatics.GetPlayerController` 0))
  (cast `/Game/Retro_Game/Blueprints/BP_CharacterBase` OtherActor)
  (`/Engine/EditorBlueprintResources/StandardMacros.IsValid` _returnvalue
    (:`Is Valid`
      (`PlayerController.SetViewTargetWithBlend` _returnvalue self 1.0 "VTBlend_Linear" 0.0 true))))

(event `self.ReceiveActorEndOverlap`
  (params (OtherActor :type "Actor Object Reference"))
  (bind _returnvalue (`GameplayStatics.GetPlayerController` 0))
  (bind _asbp_character_base (cast `/Game/Retro_Game/Blueprints/BP_CharacterBase` OtherActor))
  (`/Engine/EditorBlueprintResources/StandardMacros.IsValid` _returnvalue
    (:`Is Valid`
      (`PlayerController.SetViewTargetWithBlend` _returnvalue _asbp_character_base 1.0 "VTBlend_Linear" 0.0 true))))

(fn `ForceFocusOnFirstSpawn`
  (bind _playercast (`self.PlayerCast`))
  (`/Engine/EditorBlueprintResources/StandardMacros.IsValid` _playercast
    (:`Is Valid`
      (if (`PrimitiveComponent.IsOverlappingActor` (`self.Box`) _playercast)
        (`/Engine/EditorBlueprintResources/StandardMacros.DoOnce` false
          (:`Completed`
            (`PlayerController.SetViewTargetWithBlend` (`GameplayStatics.GetPlayerController` 0) self 0.0 "VTBlend_Linear" 0.0 false)))))))

(fn `UserConstructionScript`
  (bind _camera (`self.Camera`))
  (`SceneComponent.SetWorldScale3D` (`self.Box`) (`KismetMathLibrary.MakeVector` (`self.CollisionScaleX`) 1.0 (`self.CollisionScaleZ`)))
  (`CameraComponent.SetOrthoWidth` _camera (`self.CameraDistance`))
  (`SceneComponent.K2_SetRelativeLocation` _camera (`self.CameraLocation`) false false))