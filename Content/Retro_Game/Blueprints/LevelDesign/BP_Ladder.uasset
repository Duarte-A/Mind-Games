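; BP_Ladder is a level design ladder actor that lets overlapping BP_CharacterBase characters climb.
; Beginning overlap sets the character's CanClimb flag, while ending overlap clears it and calls StopClimbing.
; A looping timer, started and cleared with the overlap, re-enables CanClimb on player character 0, since shooting on a ladder makes the player let go and fall.
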(event `DoubleCheckCanClimb`
  ;[1 1 1] Used for when the playert shoots while on ladders, by default it will let go of the ladder and fall down, this checks if it's still overlapping with ther ladder so that climbing can be activated again
  (bind _asbp_character_base (cast `/Game/Retro_Game/Blueprints/BP_CharacterBase` (`GameplayStatics.GetPlayerCharacter` 0)))
  (set `/Game/Retro_Game/Blueprints/BP_CharacterBase.bCanClimb` true _asbp_character_base))

(event `self.ReceiveActorBeginOverlap`
  (params (OtherActor :type "Actor Object Reference"))
  (bind _asbp_character_base (cast `/Game/Retro_Game/Blueprints/BP_CharacterBase` OtherActor))
  (set `/Game/Retro_Game/Blueprints/BP_CharacterBase.bCanClimb` true _asbp_character_base)
  ;[1 1 1] Used for when the playert shoots while on ladders, by default it will let go of the ladder and fall down, this checks if it's still overlapping with ther ladder so that climbing can be activated again
  (`KismetSystemLibrary.K2_SetTimer` null "DoubleCheckCanClimb" 0.5 true))

(event `self.ReceiveActorEndOverlap`
  (params (OtherActor :type "Actor Object Reference"))
  (bind _asbp_character_base (cast `/Game/Retro_Game/Blueprints/BP_CharacterBase` OtherActor))
  (set `/Game/Retro_Game/Blueprints/BP_CharacterBase.bCanClimb` false _asbp_character_base)
  (`/Game/Retro_Game/Blueprints/BP_CharacterBase.StopClimbing` _asbp_character_base)
  ;[1 1 1] Used for when the playert shoots while on ladders, by default it will let go of the ladder and fall down, this checks if it's still overlapping with ther ladder so that climbing can be activated again
  (`KismetSystemLibrary.K2_ClearTimer` null "DoubleCheckCanClimb"))

(fn `UserConstructionScript`)