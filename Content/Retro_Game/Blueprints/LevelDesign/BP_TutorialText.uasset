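; BP_TutorialText is a level-design actor that shows in-world tutorial text to the player.
; The construction script applies the configurable text and color to a TextRender component and hides it unless AlwaysVisible is set.
; When not always visible, actor overlap events show the text while a BP_CharacterBase is overlapping and hide it when the character leaves.
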(event `self.ReceiveActorBeginOverlap`
  (params (OtherActor :type "Actor Object Reference"))
  (if (not (`self.AlwaysVisible`))
    (cast `/Game/Retro_Game/Blueprints/BP_CharacterBase` OtherActor)
    (`SceneComponent.SetVisibility` (`self.TextRender`) true false)))

(event `self.ReceiveActorEndOverlap`
  (params (OtherActor :type "Actor Object Reference"))
  (if (not (`self.AlwaysVisible`))
    (cast `/Game/Retro_Game/Blueprints/BP_CharacterBase` OtherActor)
    (`SceneComponent.SetVisibility` (`self.TextRender`) false false)))

(fn `UserConstructionScript`
  (bind _textrender (`self.TextRender`))
  (`TextRenderComponent.K2_SetText` _textrender (`self.Text`))
  (`TextRenderComponent.SetTextRenderColor` _textrender (`self.TextColor`))
  (if (not (`self.AlwaysVisible`))
    (`SceneComponent.SetVisibility` _textrender false false)))