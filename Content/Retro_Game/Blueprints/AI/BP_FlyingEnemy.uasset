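; BP_FlyingEnemy is a Paper2D enemy that patrols between two points, fires projectiles on a looping timer and damages the player character on overlap.
; A timeline lerps the flipbook to EndLocation and back, pausing at each end, while the construction script can preview that endpoint.
; Damage drains Health; death spawns a random pickup, stops firing, disables box collision and plays an explosion flipbook before destroying the actor.
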(event `self.ReceiveBeginPlay`
  (`self.Play`)
  (`KismetSystemLibrary.K2_SetTimer` null "FireProjectile" 0.5 true))

(event `Play`
  (bind (_direction _alpha) (`Timeline|MovePlatform_TL` :!label _label)
    (:`Update`
      (`SceneComponent.K2_SetRelativeLocation` (`self.PaperFlipbook`) (`KismetMathLibrary.VLerp` (0.0 0.0 0.0) (`self.End_Location`) _alpha) false false))
    (:`Finished`
      (`KismetSystemLibrary.Delay` (`self.Stop_Delay`))
      (switch `ETimelineDirection` _direction
        (:`Forward`
          (`self.Reverse`))
        (:`Backward`
          (`self.Play`))))))

(event `Reverse`
  (goto _label :!via `Reverse`))

(event `self.ReceiveAnyDamage`
  (params (Damage :type "Float (single-precision)") (DamageType :type "DamageType Object Reference") (InstigatedBy :type "Controller Object Reference") (DamageCauser :type "Actor Object Reference"))
  (bind _paperflipbook (`self.PaperFlipbook`))
  (bind _output_get (set `self.Health` (- (`self.Health`) Damage)))
  (if (<= _output_get 0.0)
    (`/Engine/EditorBlueprintResources/StandardMacros.DoOnce` false
      (:`Completed`
        (`|SpawnActorFromClass` "/Game/Retro_Game/Blueprints/PickUps/BP_SpawnRandomPickUp.BP_SpawnRandomPickUp_C" (`KismetMathLibrary.MakeTransform` (`SceneComponent.K2_GetComponentLocation` (`self.PaperFlipbook`))) "AlwaysSpawn" "OverrideRootScale" null null)
        (`KismetSystemLibrary.K2_ClearTimer` null "FireProjectile")
        (`PrimitiveComponent.SetCollisionEnabled` (`self.Box`) "NoCollision")
        (`GameplayStatics.SpawnSoundAtLocation` "/Game/Retro_Game/Sounds/SFX_GotHit.SFX_GotHit" (`self.K2_GetActorLocation`) (struct) 1.0 1.0 0.0 null null)
        (`PaperFlipbookComponent.SetFlipbook` _paperflipbook "/Game/Retro_Game/Sprites/FlipBooks/Explosion/F_Explosion.F_Explosion")
        (`KismetSystemLibrary.Delay` (`PaperFlipbookComponent.GetFlipbookLength` _paperflipbook))
        (`self.K2_DestroyActor`)))
    (else
      (`GameplayStatics.SpawnSoundAtLocation` "/Game/Retro_Game/Sounds/SFX_EnemyHit_Cue.SFX_EnemyHit_Cue" (`self.K2_GetActorLocation`) (struct) 1.0 1.0 0.0 null null))))

(event `self.ReceiveActorBeginOverlap`
  (params (OtherActor :type "Actor Object Reference"))
  (bind _asbp_character_base (cast `/Game/Retro_Game/Blueprints/BP_CharacterBase` OtherActor))
  (`GameplayStatics.ApplyDamage` _asbp_character_base 0.1))

(event `FireProjectile`
  (bind _arrow (`self.Arrow`))
  (`|SpawnActorFromClass` "/Game/Retro_Game/Blueprints/AI/BP_Enemy_Projectile.BP_Enemy_Projectile_C" (`KismetMathLibrary.MakeTransform` (`SceneComponent.K2_GetComponentLocation` _arrow) (`SceneComponent.K2_GetComponentRotation` _arrow)) "AlwaysSpawn" "OverrideRootScale" null 0.2 0.5 null))

(fn `UserConstructionScript`
  (bind _end_location (`self.End_Location`))
  (set `self.End_Location` _end_location)
  (`SceneComponent.K2_SetRelativeLocation` (`self.PaperFlipbook`) (select `bool` (`self.Test_EndLocation`) :`true` _end_location) false false))