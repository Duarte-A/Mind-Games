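; Configurable base for 2D flipbook enemies that patrol between two points, attack the player character and take damage.
; A timeline lerps the sprite to EndLocation and back, optionally flipping it and pausing for melee or firing animations.
; Projectiles fire on a gated repeat loop or during turnaround stops.
; Overlap damages characters; hits flicker a dynamic material, and death or explode-on-touch plays an explosion, spawns loot and destroys the actor.
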(event `self.ReceiveBeginPlay`
  (`TimelineComponent.SetPlayRate` (`self.MovementTimeline`) (/ 1.0 (`self.TimeSeconds`)))
  (set `self.TestEndLocation` false)
  (if (`self.canFire`)
    (if (not (`self.StopMovementWhileFiring`))
      (`self.FireProjectile`))))

(event `self.ReceiveActorEndOverlap`
  (params (OtherActor :type "Actor Object Reference"))
  (cast `/Game/Retro_Game/Blueprints/BP_CharacterBase` OtherActor)
  (if (`self.isMeleeAttacking`)
    (set `self.isMeleeAttacking` false)))

(event `self.ReceiveActorBeginOverlap`
  (params (OtherActor :type "Actor Object Reference"))
  (bind _meleeflipbook (`self.MeleeFlipbook`))
  (bind _flipbook (`self.Flipbook`))
  (bind _laser (`self.Laser`))
  (bind _returnvalue_location (`KismetMathLibrary.BreakTransform` (`KismetMathLibrary.Conv_VectorToTransform` (`SceneComponent.K2_GetComponentLocation` (`self.Flipbook`)))))
  (bind (_returnvalue_location_2 _returnvalue_rotation) (`KismetMathLibrary.BreakTransform` (`KismetMathLibrary.Conv_VectorToTransform` (`SceneComponent.K2_GetComponentLocation` (`self.Flipbook`)))))
  (bind _asbp_character_base (cast `/Game/Retro_Game/Blueprints/BP_CharacterBase` OtherActor))
  (if (`self.CanMeleeAttack`)
    (set `self.isMeleeAttacking` true)
    (`SceneComponent.SetVisibility` (`self.Flipbook`) false false)
    (`SceneComponent.SetVisibility` _meleeflipbook true false)
    (`|ExecutionSequence`
      (:`then_0`
        (bind _output_get (set `self.MeleeDelay` (`PaperFlipbookComponent.GetFlipbookLength` _meleeflipbook)))
        (`KismetSystemLibrary.Delay` _output_get)
        (`SceneComponent.SetVisibility` (`self.Flipbook`) true false)
        (`SceneComponent.SetVisibility` (`self.MeleeFlipbook`) false false)
        (set `self.isMeleeAttacking` false))
      (:`then_1`
        (if (`Actor.bCanBeDamaged` _asbp_character_base) :!label _label
          (`GameplayStatics.ApplyDamage` _asbp_character_base (`self.Damage`))
          (if (`self.ExplodeOnTouch`)
            (`|SpawnActorFromClass` "/Game/Retro_Game/Blueprints/PickUps/BP_SpawnRandomPickUp.BP_SpawnRandomPickUp_C" (`KismetMathLibrary.MakeTransform` _returnvalue_location_2 _returnvalue_rotation) "AlwaysSpawn" "OverrideRootScale" null null)
            (`PaperFlipbookComponent.SetFlipbook` _flipbook (`self.EnemyDeathExplosion`) :!label _label_2)
            (if (`self.isMeleeAttacking`)
              (`SceneComponent.SetVisibility` (`self.MeleeFlipbook`) false false)
              (`SceneComponent.SetVisibility` (`self.Flipbook`) true false)
              (elif (`self.StopMovementWhileFiring`)
                (`SceneComponent.SetVisibility` (`self.FiringFlipbook`) false false)
                (`SceneComponent.SetVisibility` (`self.Flipbook`) true false)))
            (`PrimitiveComponent.SetCollisionEnabled` (`self.CollisionBox`) "NoCollision")
            (`SceneComponent.SetWorldScale3D` _flipbook (`self.EnemyDeathExplosionScale`))
            (`self.TimelineStop`)
            (`GameplayStatics.SpawnSoundAttached` (`self.EnemyDeathSound`) (`self.Flipbook`) "None" (0.0 0.0 0.0) (struct) "KeepRelativeOffset" false 1.0 1.0 0.0 null null)
            (`/Engine/EditorBlueprintResources/StandardMacros.DoOnce` false
              (:`Completed`
                (`|SpawnActorFromClass` (`self.LootSpawner`) (`KismetMathLibrary.MakeTransform` _returnvalue_location) "AlwaysSpawn" "SelectDefaultAtRuntime" null null)
                (if (`self.isLaserProjectile`)
                  (`/Engine/EditorBlueprintResources/StandardMacros.IsValid` _laser
                    (:`Is Valid`
                      (`self.K2_DestroyActor` _laser)
                      (`KismetSystemLibrary.Delay` (`PaperFlipbookComponent.GetFlipbookLength` (`self.Flipbook`)) :!label _label_3))
                    (:`Is Not Valid`
                      _))
                  (else
                    (goto _label_3)))
                (`self.K2_DestroyActor`)))))))
    (else
      (goto _label))))

(event `self.ReceiveAnyDamage`
  (params (Damage :type "Float (single-precision)") (DamageType :type "DamageType Object Reference") (InstigatedBy :type "Controller Object Reference") (DamageCauser :type "Actor Object Reference"))
  (`MaterialInstanceDynamic.SetScalarParameterValue` (`self.SpriteDynMat`) "Flicker" 1.0)
  (if (`self.canBeDamaged`)
    (bind _output_get (set `self.EnemyHealth` (- (`self.EnemyHealth`) Damage)))
    (if (<= _output_get 0.0)
      (goto _label_2)
      (else
        (`GameplayStatics.SpawnSoundAttached` (`self.EnemyGotHitSound`) (`self.Flipbook`) "None" (0.0 0.0 0.0) (struct) "KeepRelativeOffset" false 1.0 1.0 0.0 null null)
        (`KismetSystemLibrary.Delay` 0.2)
        (`MaterialInstanceDynamic.SetScalarParameterValue` (`self.SpriteDynMat`) "Flicker" 0.0)))
    (else
      (`GameplayStatics.SpawnSoundAttached` null (`self.Flipbook`) "None" (0.0 0.0 0.0) (struct) "KeepRelativeOffset" false 1.0 1.0 0.0 null null)
      (`MaterialInstanceDynamic.SetScalarParameterValue` (`self.SpriteDynMat`) "Flicker" 0.0))))

(event `FireProjectile`
  (bind (_returnvalue_location _returnvalue_rotation) (`KismetMathLibrary.BreakTransform` (`SceneComponent.K2_GetComponentToWorld` (`self.Arrow`))))
  (if (`self.StopMovementWhileFiring`)
    (`|ExecutionSequence` :!label _label_4
      (:`then_1`
        _)
      (:`then_2`
        (`KismetSystemLibrary.RetriggerableDelay` (`self.ProjectileFirerate`))
        (`/Engine/EditorBlueprintResources/StandardMacros.Gate` true :!label _label_5
          (:`Exit`
            (goto _label_4)))))
    (else
      (`|ExecutionSequence`
        (:`then_0`
          (goto _label_5 :!via `Open`))
        (:`then_1`
          (goto _label_5)))))
  (bind _returnvalue (`|SpawnActorFromClass` (`self.EnemyProjectile`) (`KismetMathLibrary.MakeTransform` _returnvalue_location _returnvalue_rotation) "AlwaysSpawn" "SelectDefaultAtRuntime" null null))
  (if (`self.isLaserProjectile`)
    (set `self.Laser` _returnvalue)))

(event `TimelinePlayFromStart`
  (bind _firingflipbook (`self.FiringFlipbook`))
  (bind _flipbook (`self.Flipbook`))
  (bind (_direction _flyalhpa) (`Timeline|MovementTimeline` :!via `PlayFromStart` :!label _label_6)
    (:`Update`
      (if (`self.isMeleeAttacking`)
        (`self.TimelineStop`)
        (`KismetSystemLibrary.Delay` (`self.MeleeDelay`))
        (if (`self.MoveDirection`)
          (`self.TimelineReverse`)
          (else
            (`self.TimelinePlay`)))
        (else
          (`SceneComponent.K2_SetRelativeLocation` (`self.Flipbook`) (`KismetMathLibrary.VLerp` (0.0 0.0 0.0) (`self.EndLocation`) _flyalhpa) false false))))
    (:`Finished`
      (if (`self.StopMovementWhileFiring`)
        (`SceneComponent.SetVisibility` (`self.Flipbook`) false false)
        (`SceneComponent.SetVisibility` _firingflipbook true false)
        (bind _output_get (set `self.FiringAnimationDelay` (`PaperFlipbookComponent.GetFlipbookLength` _firingflipbook)))
        (`/Engine/EditorBlueprintResources/StandardMacros.DoOnce` false :!label _label_7
          (:`Completed`
            (`self.FireProjectile`)
            (`KismetSystemLibrary.Delay` _output_get)
            (`SceneComponent.SetVisibility` (`self.Flipbook`) true false)
            (`SceneComponent.SetVisibility` (`self.FiringFlipbook`) false false))))
      (`KismetSystemLibrary.Delay` (`self.PauseBeforeChangingDirection`))
      (switch `ETimelineDirection` _direction
        (:`Forward`
          (`self.TimelineReverseFromEnd`)
          (if (`self.FlipSprite`)
            (`SceneComponent.K2_SetWorldRotation` _flipbook (struct :`Yaw` 180.0) false false)
            (set `self.MoveDirection` true)
            (`self.ResetSpawnProj` :!label _label_8)))
        (:`Backward`
          (`self.TimelinePlayFromStart`)
          (if (`self.FlipSprite`)
            (`SceneComponent.K2_SetWorldRotation` :`self` _flipbook)
            (set `self.MoveDirection` false)
            (goto _label_8)))))))

(event `TimelineReverseFromEnd`
  (goto _label_6 :!via `ReverseFromEnd`))

(event `TimelineStop`
  (goto _label_6 :!via `Stop`))

(event `TimelinePlay`
  (goto _label_6))

(event `TimelineReverse`
  (goto _label_6 :!via `Reverse`))

(event `ResetSpawnProj`
  (goto _label_7 :!via `Reset`))

(fn `UserConstructionScript`
  (`SceneComponent.K2_SetRelativeLocation` (`self.Flipbook`) (`KismetMathLibrary.SelectVector` (`self.EndLocation`) (0.0 0.0 0.0) (`self.TestEndLocation`)) false false)
  (`PaperFlipbookComponent.SetFlipbook` (`self.Flipbook`) (`self.EnemySprite_Flipbook`))
  (`PaperFlipbookComponent.SetFlipbook` (`self.MeleeFlipbook`) (`self.MeleeSprite`))
  (`PaperFlipbookComponent.SetFlipbook` (`self.FiringFlipbook`) (`self.FiringSprite`))
  (`SceneComponent.SetRelativeScale3D` (`self.CollisionBox`) (`self.CollisionBoxScale`))
  (bind _returnvalue (`PrimitiveComponent.CreateDynamicMaterialInstance` (`self.Flipbook`) 0 null "None"))
  (set `self.SpriteDynMat` _returnvalue))