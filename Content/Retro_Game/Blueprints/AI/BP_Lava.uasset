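; Lava hazard actor for the retro game that slows and damages the player character while it overlaps the lava.
; Overlap begin turns on the character's slowdown, deals damage at once and starts a looping timer for repeat hits; overlap end undoes the slowdown and clears the timer.
; Damage always targets player 0's character cached at BeginPlay, whichever BP_CharacterBase triggered the overlap.
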(event `self.ReceiveBeginPlay`
  (bind _asbp_character_base (cast `/Game/Retro_Game/Blueprints/BP_CharacterBase` (`GameplayStatics.GetPlayerCharacter` 0)))
  (set `self.PlayerCast` _asbp_character_base))

(event `self.ReceiveActorBeginOverlap`
  (params (OtherActor :type "Actor Object Reference"))
  (bind _asbp_character_base (cast `/Game/Retro_Game/Blueprints/BP_CharacterBase` OtherActor))
  (`/Game/Retro_Game/Blueprints/BP_CharacterBase.Slowdown` _asbp_character_base true)
  (`self.DamageOverTime`)
  (`KismetSystemLibrary.K2_SetTimer` null "DamageOverTime" 1.2 true))

(event `self.ReceiveActorEndOverlap`
  (params (OtherActor :type "Actor Object Reference"))
  (bind _asbp_character_base (cast `/Game/Retro_Game/Blueprints/BP_CharacterBase` OtherActor))
  (`/Game/Retro_Game/Blueprints/BP_CharacterBase.Slowdown` _asbp_character_base false)
  (`KismetSystemLibrary.K2_ClearTimer` null "DamageOverTime"))

(event `DamageOverTime`
  (`GameplayStatics.ApplyDamage` (`self.PlayerCast`) 0.1))

(fn `UserConstructionScript`)