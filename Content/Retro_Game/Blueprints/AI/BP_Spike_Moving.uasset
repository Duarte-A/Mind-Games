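; BP_Spike_Moving is a moving spike hazard that damages characters on overlap.
; A timeline starts on BeginPlay and moves the box and sprite between start and end positions, pausing a second at each end before reversing.
; Any overlapping BP_CharacterBase receives one point of damage.
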(event `self.ReceiveBeginPlay`
  (`self.Play`))

(event `Play`
  (bind (_direction _alpha) (`Timeline|MoveSpike` :!label _label)
    (:`Update`
      (`SceneComponent.K2_SetRelativeLocation` (`self.Box`) (`KismetMathLibrary.VLerp` (`self.StartPosition`) (`self.EndPosition`) _alpha) false false)
      (`SceneComponent.K2_SetRelativeLocation` (`self.PaperSprite`) (`KismetMathLibrary.VLerp` (`self.StartPosition`) (`self.EndPosition`) _alpha) false false))
    (:`Finished`
      (`KismetSystemLibrary.Delay` 1.0)
      (switch `ETimelineDirection` _direction
        (:`Forward`
          (`self.Reverse`))
        (:`Backward`
          (`self.Play`))))))

(event `Reverse`
  (goto _label :!via `Reverse`))

(event `self.ReceiveActorBeginOverlap`
  (params (OtherActor :type "Actor Object Reference"))
  (bind _asbp_character_base (cast `/Game/Retro_Game/Blueprints/BP_CharacterBase` OtherActor))
  (`GameplayStatics.ApplyDamage` _asbp_character_base 1.0 null self))

(fn `UserConstructionScript`)