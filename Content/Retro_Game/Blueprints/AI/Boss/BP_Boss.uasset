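; Retro game boss that patrols, shoots and loads the Ending level on death.
; A timeline ping-pongs its flipbook toward EndLocation with pauses, previewable in the construction script, while a looping timer fires projectiles from an arrow.
; Damage updates a widget health bar, and box overlap hurts characters.
; At zero health, a one-shot sequence stops firing, plays sound, flickers via dynamic material and swaps to explosion before destroying the actor.
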(event `self.ReceiveBeginPlay`
  (`self.Play`)
  (`self.UpdateBossHealthWidget`)
  (`KismetSystemLibrary.K2_SetTimer` null "FireProjectile" 0.2 true))

(event `Play`
  (bind (_direction _alpha) (`Timeline|MovingTimeline` :!label _label)
    (:`Update`
      (`SceneComponent.K2_SetRelativeLocation` (`self.PaperFlipbook`) (`KismetMathLibrary.VLerp` (0.0 0.0 0.0) (`self.End_Location`) _alpha) false false))
    (:`Finished`
      (`KismetSystemLibrary.Delay` (`self.Stop_Delay`))
      (switch `ETimelineDirection` _direction
        (:`Forward`
          (`self.Reverse`))
        (:`Backward`
          (`self.Play`))))))

(event `Reverse`
  (goto _label :!via `Reverse`))

(event `self.ReceiveAnyDamage`
  (params (Damage :type "Float (single-precision)") (DamageType :type "DamageType Object Reference") (InstigatedBy :type "Controller Object Reference") (DamageCauser :type "Actor Object Reference"))
  (bind _output_get (set `self.Health` (- (`self.Health`) Damage)))
  (if (<= _output_get 0.0)
    (`/Engine/EditorBlueprintResources/StandardMacros.DoOnce` false
      (:`Completed`
        (`KismetSystemLibrary.K2_ClearTimer` null "FireProjectile")
        (`GameplayStatics.SpawnSoundAtLocation` "/Game/Retro_Game/Sounds/SFX_Explosion_Cue.SFX_Explosion_Cue" (`self.K2_GetActorLocation`) (struct) 1.0 1.0 0.0 null null)
        (`SceneComponent.SetVisibility` (`self.Widget`) false false)
        (`MaterialInstanceDynamic.SetScalarParameterValue` (`self.FlickerMaterial`) "Flicker" 1.0)
        (`PaperFlipbookComponent.SetFlipbook` (`self.PaperFlipbook`) "/Game/Retro_Game/Sprites/FlipBooks/Boss/F_Enemy_Boss_02.F_Enemy_Boss_02")
        (`KismetSystemLibrary.Delay` 3.0)
        (`PaperFlipbookComponent.SetFlipbook` (`self.PaperFlipbook`) "/Game/Retro_Game/Sprites/FlipBooks/Explosion/F_Explosion.F_Explosion")
        (`KismetSystemLibrary.Delay` 1.0)
        (`self.K2_DestroyActor`)
        (`GameplayStatics.OpenLevel` "Ending")))
    (else
      (`self.UpdateBossHealthWidget`))))

(event `UpdateBossHealthWidget`
  (bind _asw_boss_health_bar (cast `/Game/Retro_Game/Blueprints/AI/Boss/W_BossHealthBar` (`WidgetComponent.GetUserWidgetObject` (`self.Widget`))))
  (`ProgressBar.SetPercent` (`/Game/Retro_Game/Blueprints/AI/Boss/W_BossHealthBar.Boss_HealthBar` _asw_boss_health_bar) (/ (`self.Health`) (`self.Health_Max`))))

(event `FireProjectile`
  (bind _arrow (`self.Arrow`))
  (`|SpawnActorFromClass` "/Game/Retro_Game/Blueprints/AI/BP_Enemy_Projectile.BP_Enemy_Projectile_C" (`KismetMathLibrary.MakeTransform` (`SceneComponent.K2_GetComponentLocation` _arrow) (`SceneComponent.K2_GetComponentRotation` _arrow)) "AlwaysSpawn" "OverrideRootScale" null 0.1 1.0 null))

(event `self.Box.OnComponentBeginOverlap`
  (params (OverlappedComponent :type "PrimitiveComponent Object Reference") (OtherActor :type "Actor Object Reference") (OtherComp :type "PrimitiveComponent Object Reference") (OtherBodyIndex :type Integer) (bFromSweep :type Boolean) (SweepResult :type "HitResult Structure (by ref)"))
  (bind _asbp_character_base (cast `/Game/Retro_Game/Blueprints/BP_CharacterBase` OtherActor))
  (`GameplayStatics.ApplyDamage` _asbp_character_base 0.2))

(fn `UserConstructionScript`
  (bind _end_location (`self.End_Location`))
  (bind _paperflipbook (`self.PaperFlipbook`))
  (set `self.End_Location` _end_location)
  (`SceneComponent.K2_SetRelativeLocation` _paperflipbook (select `bool` (`self.Test_EndLocation`) :`true` _end_location) false false)
  (bind _returnvalue (`PrimitiveComponent.CreateDynamicMaterialInstance` _paperflipbook 0 "/Game/Retro_Game/Sprites/Materials/DefaultSpriteMaterialFLICKER.DefaultSpriteMaterialFLICKER" "None"))
  (set `self.FlickerMaterial` _returnvalue))